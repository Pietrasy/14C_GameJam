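; Player controller that maps Enhanced Input to character movement and camera look, with head-bob camera shakes.
; BeginPlay adds the default mapping context and starts the idle bob.
; Movement follows control rotation, starting the walking shake on every trigger, then stopping the last stored shake and restarting idle on completion.
; Look input passes through FInterpTo from InputAxisX/Y, which are never updated here, before feeding yaw and pitch.
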(event `self.ReceiveBeginPlay`
  (`EnhancedInputSubsystemInterface.AddMappingContext` (subsystem `EnhancedInputLocalPlayerSubsystem`) "/Game/Input/IMC_Default.IMC_Default" 0 (struct))
  (`self.PlayCameraShake` "/Game/Blueprints/Misc/CameraShakes/CamShake_HeadBob_Idle.CamShake_HeadBob_Idle_C"))

(event `EnhancedInput|/Game/Input/Actions/IA_Move`
  (params (ActionValue :type "Vector2D Structure") (ElapsedSeconds :type "Float (double-precision)") (TriggeredSeconds :type "Float (double-precision)") (InputAction :type "InputAction Object Reference" :default "/Game/Input/Actions/IA_Move.IA_Move"))
  (:`Triggered`
    (`Pawn.AddMovementInput` (`GameplayStatics.GetPlayerCharacter` 0) (`KismetMathLibrary.GetForwardVector` (`self.GetControlRotation`)) ActionValue_Y false)
    (`Pawn.AddMovementInput` (`GameplayStatics.GetPlayerCharacter` 0) (`KismetMathLibrary.GetRightVector` (`self.GetControlRotation`)) ActionValue_X false)
    (`self.PlayCameraShake` "/Game/Blueprints/Misc/CameraShakes/CamShake_HeadBob_Walking.CamShake_HeadBob_Walking_C"))
  (:`Completed`
    (`PlayerCameraManager.StopCameraShake` (`GameplayStatics.GetPlayerCameraManager` 0) (`self.CameraShakeInstance`) false)
    (`self.PlayCameraShake` "/Game/Blueprints/Misc/CameraShakes/CamShake_HeadBob_Idle.CamShake_HeadBob_Idle_C")))

(event `EnhancedInput|/Game/Input/Actions/IA_Look`
  (params (ActionValue :type "Vector2D Structure") (ElapsedSeconds :type "Float (double-precision)") (TriggeredSeconds :type "Float (double-precision)") (InputAction :type "InputAction Object Reference" :default "/Game/Input/Actions/IA_Look.IA_Look"))
  (:`Triggered`
    (`self.LookLeftRight` ActionValue_X)
    (`self.LookUpDown` ActionValue_Y)))

(fn `LookLeftRight`
  (params (ValueX :type "Float (double-precision)"))
  (`self.AddYawInput` (`KismetMathLibrary.FInterpTo` (`self.InputAxisX`) ValueX (`GameplayStatics.GetWorldDeltaSeconds`) 90.0)))

(fn `LookUpDown`
  (params (ValueY :type "Float (double-precision)"))
  (`self.AddPitchInput` (`KismetMathLibrary.FInterpTo` (`self.InputAxisY`) ValueY (`GameplayStatics.GetWorldDeltaSeconds`) 90.0)))

(fn `PlayCameraShake`
  (params (ShakeClass :type "CameraShakeBase Class Reference"))
  (bind _returnvalue (`PlayerCameraManager.StartCameraShake` :`self` (`GameplayStatics.GetPlayerCameraManager` 0) :`ShakeClass` (`local.ShakeClass`)))
  (set `self.CameraShakeInstance` _returnvalue))

(fn `UserConstructionScript`)