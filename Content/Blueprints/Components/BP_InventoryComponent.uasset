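; BP_InventoryComponent is an inventory component that keeps pickable items in an Inventory array.
; It exposes functions to add and remove a given pickable.
; A lookup function scans the array linearly and returns the first item whose class exactly matches the requested pickup class, or nothing when none matches.
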(fn `AddToInventory`
  (params (Pickable :type "/Game/Blueprints/Actors/Pickables/BP_PickableBase Object Reference"))
  (`KismetArrayLibrary.Array_Add` (`self.Inventory`) Pickable)
  (return))

(fn `FindItemFromInventory`
  (params (PickupClass :type "/Game/Blueprints/Actors/Pickables/BP_PickableBase Class Reference"))
  (returns (Pickup :type "/Game/Blueprints/Actors/Pickables/BP_PickableBase Object Reference"))
  (locals (PickupFromArray :type "/Game/Blueprints/Actors/Pickables/BP_PickableBase Object Reference"))
  (for _array_element (`self.Inventory`)
    (bind _output_get (set `local.PickupFromArray` _array_element))
    (if (== (`GameplayStatics.GetObjectClass` _output_get) (`local.PickupClass`))
      (return (`local.PickupFromArray`))))
  (return null))

(fn `RemoveFromInventory`
  (params (Pickable :type "/Game/Blueprints/Actors/Pickables/BP_PickableBase Object Reference"))
  (`KismetArrayLibrary.Array_RemoveItem` (`self.Inventory`) Pickable)
  (return))