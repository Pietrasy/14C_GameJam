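; Actor component that detects what its owning player character looks at, for interaction.
; On BeginPlay it caches the owner, and CastTraceToInteract gets that character's camera through GetCameraComponentMessage.
; It then line traces forward from the camera up to Range on TraceTypeQuery3 and broadcasts OnDetectInteraction with the hit result when something is struck.
; The trace does not run on its own, as nothing in this component calls it.
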(event `self.ReceiveBeginPlay`
  (`self.CachePlayerCharacter`))

(fn `CachePlayerCharacter`
  (set `self.PlayerCharacter` (`self.GetOwner`)))

(fn `CastTraceToInteract`
  (locals (HitInfo :type "HitResult Structure") (ActorLocation :type "Vector Structure" :default (0.0 0.0 0.0)) (ActorCamera :type "CameraComponent Object Reference"))
  (bind _playercharacter (`self.PlayerCharacter`)
    (:`then`
      (bind _cameracomponent (message `/Game/Blueprints/Interfaces/BPI_Player.GetCameraComponent` _playercharacter))
      (bind _output_get (set `local.ActorCamera` _cameracomponent))
      (bind _output_get_2 (set `local.ActorLocation` (`SceneComponent.K2_GetComponentLocation` _output_get)))
      (bind (_outhit _returnvalue) (`KismetSystemLibrary.LineTraceSingle` _output_get_2 (+ (`local.ActorLocation`) (* (`KismetMathLibrary.Conv_RotatorToVector` (`SceneComponent.K2_GetComponentRotation` (`local.ActorCamera`))) (`self.Range`))) "TraceTypeQuery3"))
      (set `local.HitInfo` _outhit)
      (if _returnvalue
        (`self.OnDetectInteraction` (`local.HitInfo`))
        (return)))
    (:`else`)))