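; Interactable door actor that moves the player between streamed levels when active.
; On interact it disables input, fires the OnNewLevel dispatcher, shows the HUD loading screen and asynchronously loads LevelToLoad.
; Once loaded, it hides the screen, messages the player character with the SpawnLocation position, restores input and unloads CurrentLevel.
; The sound playback nodes are never run.
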(event `/Game/Blueprints/Interfaces/BPI_Interactable.Interact`
  (params (Interactor :type "Actor Object Reference"))
  (set `self.Interactor` Interactor)
  (if (`self.IsActive`)
    (`self.DisableInput` (`GameplayStatics.GetPlayerController` 0))
    (`self.OnNewLevel`)
    (message `/Game/Blueprints/Interfaces/BPI_HUD.DisplayLoadingScreen` (`PlayerController.GetHUD` (`GameplayStatics.GetPlayerController` 0)))
    (`GameplayStatics.LoadStreamLevelBySoftObjectPtr` (`self.LevelToLoad`) true)
    (message `/Game/Blueprints/Interfaces/BPI_HUD.HideLoadingScreen` (`PlayerController.GetHUD` (`GameplayStatics.GetPlayerController` 0)))
    (message `/Game/Blueprints/Interfaces/BPI_Player.LocationToSpawn` (`GameplayStatics.GetPlayerCharacter` 0) (`SceneComponent.K2_GetComponentLocation` (`self.SpawnLocation`)))
    (`self.EnableInput` (`GameplayStatics.GetPlayerController` 0))
    (`GameplayStatics.UnloadStreamLevelBySoftObjectPtr` (`self.CurrentLevel`))))

(fn `UserConstructionScript`)