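; BP_LoadNewLevel is a trigger actor that moves an overlapping Character from the current streamed level into another.
; On overlap it disables input, shows WBP_LoadingScreen and loads LevelToLoad without blocking.
; It then moves the character to its Capsule component's world location, which serves as the destination marker.
; After a short fixed delay it removes the loading screen, restores input and unloads CurrentLevel.
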(event `self.ReceiveActorBeginOverlap`
  (params (OtherActor :type "Actor Object Reference"))
  (bind _ascharacter (cast `Character` OtherActor))
  (bind _returnvalue (`|CreateWidget` "/Game/Blueprints/Widgets/WBP_LoadingScreen.WBP_LoadingScreen_C"))
  (`self.DisableInput` _ascharacter (`GameplayStatics.GetPlayerController` 0))
  (`UserWidget.AddToViewport` _returnvalue 0)
  (`GameplayStatics.LoadStreamLevelBySoftObjectPtr` (`self.Level_to_Load`) true)
  (`self.K2_SetActorLocation` _ascharacter (`SceneComponent.K2_GetComponentLocation` (`self.Capsule`)) false false)
  (`KismetSystemLibrary.Delay` 1.0)
  (`Widget.RemoveFromParent` _returnvalue)
  (`self.EnableInput` _ascharacter (`GameplayStatics.GetPlayerController` 0))
  (`GameplayStatics.UnloadStreamLevelBySoftObjectPtr` (`self.Current_Level`)))

(fn `UserConstructionScript`)