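; BP_BulbSlot is an interactable slot that takes a bulb and relays a signal along a rotatable line of sight.
; Interacting while looking at it, checked by camera dot product, shows its widget and either installs a BP_Bulb from inventory or rotates the Arrow 90 degrees by timeline.
; After rotating or receiving a signal, it line-traces along the Arrow and messages RetrieveSignal to the hit actor, enabling chains.
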(event `self.ReceiveBeginPlay`
  (if (`self.IsBulbSet`)
    (`SceneComponent.SetHiddenInGame` (`self.Bulb`) false false)))

(event `/Game/Blueprints/Interfaces/BPI_Interactable.Interact`
  (params (Interactor :type "Actor Object Reference"))
  (bind _returnvalue (`self.DotProduct`))
  (if (< 0.93 _returnvalue)
    (`Widget.SetVisibility` (`WidgetComponent.GetWidget` (`self.Widget`)) "Visible")
    (set `self.IsInteractable` true)
    (else
      (`Widget.SetVisibility` (`WidgetComponent.GetWidget` (`self.Widget`)) "Collapsed")
      (set `self.IsInteractable` false)))
  (if (`self.IsInteractable`)
    (if (`self.IsBulbSet`)
      (if (not (`ActorComponent.IsActive` (`self.BulbRotation_Timeline`)))
        (set `self.PreviousRotation` 0.0)
        (bind (_direction _interpolation) (`Timeline|BulbRotation_Timeline` :!via `PlayFromStart`)
          (:`Update`
            (bind _output_get (set `self.CurrentRotation` (* _interpolation 90.0)))
            (bind _output_get_2 (set `self.DeltaRotation` (- _output_get (`self.PreviousRotation`))))
            (`SceneComponent.K2_AddLocalRotation` (`self.Arrow`) (`KismetMathLibrary.MakeRotator` 0.0 0.0 _output_get_2) false false)
            (set `self.PreviousRotation` (`self.CurrentRotation`)))
          (:`Finished`
            (`self.CastLineTraceToNextBulb`))))
      (else
        (bind _item (message `/Game/Blueprints/Interfaces/BPI_Inventory.GetItemFromInventory` Interactor "/Game/Blueprints/Actors/Pickables/BP_Bulb.BP_Bulb_C" true))
        (`/Engine/EditorBlueprintResources/StandardMacros.IsValid` _item
          (:`Is Valid`
            (`SceneComponent.SetHiddenInGame` (`self.Bulb`) false false)
            (set `self.IsBulbSet` true)))))))

(event `/Game/Blueprints/Interfaces/BPI_Bulbs.RetrieveSignal`
  (`self.CastLineTraceToNextBulb`))

(fn `CastLineTraceToNextBulb`
  (bind _returnvalue (`SceneComponent.K2_GetComponentLocation` (`self.Arrow`)))
  (bind _outhit (`KismetSystemLibrary.LineTraceSingle` :`Start` _returnvalue :`End` (+ (* (`KismetMathLibrary.Conv_RotatorToVector` (`SceneComponent.K2_GetComponentRotation` (`self.Arrow`))) 1000.0) _returnvalue) :`TraceChannel` "TraceTypeQuery1" :`DrawDebugType` "ForDuration"))
  (message `/Game/Blueprints/Interfaces/BPI_Bulbs.RetrieveSignal` (`.HitActor` (`GameplayStatics.BreakHitResult` _outhit))))

(fn `DotProduct`
  (returns (ReturnValue :type "Float (double-precision)"))
  (bind _returnvalue (`GameplayStatics.GetPlayerCameraManager` 0))
  (return (`KismetMathLibrary.Dot_VectorVector` (`self.GetActorForwardVector` _returnvalue) (`KismetMathLibrary.GetDirectionUnitVector` (`PlayerCameraManager.GetCameraLocation` _returnvalue) (`self.K2_GetActorLocation`)))))

(fn `GetDotProduct`
  (returns (Dot :type "Float (double-precision)"))
  (return 0.0))

(fn `UserConstructionScript`
  (`parent.UserConstructionScript`))