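; Missing painting interactable that takes painting pieces from the interacting actor's inventory and shows them on its frame.
; Interact calls GetAllPieces, which removes a BP_PaintingPiece from the inventory and snaps a runtime-added copy of its mesh onto the interactable mesh.
; A separate AddPieceToFrame function, uncalled in these graphs, adds a mesh and fires the all-pieces-collected dispatcher based on a piece-count comparison.
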(event `/Game/Blueprints/Interfaces/BPI_Interactable.ReceiveInteraction`
  (params (Interactor :type "Actor Object Reference")))

(event `/Game/Blueprints/Interfaces/BPI_Interactable.Interact`
  (params (Interactor :type "Actor Object Reference"))
  (`self.GetAllPieces` Interactor))

(fn `AddPieceToFrame`
  (params (PieceMesh :type "StaticMesh Object Reference"))
  (bind _returnvalue (`AddComponent|NODE_AddStaticMeshComponent-1`))
  (`StaticMeshComponent.SetStaticMesh` _returnvalue (`local.PieceMesh`))
  (if (>= (`self.RequiredNumberPieces`) (`self.PieceCounter`))
    (`self.OnCollectedAllPieces`)))

(fn `GetAllPieces`
  (params (Interactor :type "Actor Object Reference"))
  (locals (IsTrue :type Boolean :default true) (Piece :type "/Game/Blueprints/Actors/Pickables/BP_PickableBase Object Reference"))
  (while (`local.IsTrue`)
    (bind _item (message `/Game/Blueprints/Interfaces/BPI_Inventory.GetItemFromInventory` (`local.Interactor`) "/Game/Blueprints/Actors/Pickables/PicturePieces/BP_PaintingPiece.BP_PaintingPiece_C" true))
    (bind _output_get (set `local.Piece` _item))
    (bind _output_get_2 (set `local.IsTrue` (`KismetSystemLibrary.IsValid` _output_get)))
    (if _output_get_2
      (bind _returnvalue (`AddComponent|NODE_AddStaticMeshComponent-2`))
      (`StaticMeshComponent.SetStaticMesh` _returnvalue (`StaticMeshComponent.StaticMesh` (`/Game/Blueprints/Actors/Pickables/BP_PickableBase.PickableStaticMesh` (`local.Piece`))))
      (`SceneComponent.K2_AttachToComponent` _returnvalue (`self.InteractableStaticMesh`) "None" "SnapToTarget" "SnapToTarget" "SnapToTarget" true)
      (return)))
  (return))

(fn `UserConstructionScript`)