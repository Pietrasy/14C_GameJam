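; BP_WardrobeOpening is an interactable wardrobe actor with logic to swing its STWardrobeDoor component open.
; A timeline scales its Doors track to a quarter turn and applies the change since the previous update as a local roll rotation, tracked through PreviousRotation.
; No event is wired to this chain, so the door animation never runs as the graph stands.
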(fn `UserConstructionScript`)