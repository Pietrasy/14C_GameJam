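; BP_Furnance is an interactable furnace that triggers the game's ending when fed coal.
; It plays a fireplace sound attached to its sphere collision from BeginPlay and stops it when destroyed.
; Interact requests and removes a BP_Coal from the player's inventory, then tells the camera manager to start the ending.
; Without coal, a DoOnce shows a HUD narrative message and calls OnDisplayMessage only the first time.
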(event `self.ReceiveBeginPlay`
  (bind _returnvalue (`GameplayStatics.SpawnSoundAttached` "/Game/Art/Sounds/A_Fireplace.A_Fireplace" (`self.SphereCollision`) "None" (0.0 0.0 0.0) (struct) "KeepRelativeOffset" false 1.0 1.0 0.0 null null))
  (set `self.FireplaceSoundInstance` _returnvalue))

(event `self.ReceiveDestroyed`
  (`AudioComponent.Stop` (`self.FireplaceSoundInstance`)))

(event `/Game/Blueprints/Interfaces/BPI_Interactable.Interact`
  (params (Interactor :type "Actor Object Reference"))
  (bind _item (message `/Game/Blueprints/Interfaces/BPI_Inventory.GetItemFromInventory` (`GameplayStatics.GetPlayerCharacter` 0) "/Game/Blueprints/Actors/Pickables/BP_Coal.BP_Coal_C" true))
  (`/Engine/EditorBlueprintResources/StandardMacros.IsValid` _item
    (:`Is Valid`
      (message `/Game/Blueprints/Interfaces/BPI_CameraManager.StartEnding` (`GameplayStatics.GetPlayerCameraManager` 0)))
    (:`Is Not Valid`
      (`/Engine/EditorBlueprintResources/StandardMacros.DoOnce` false
        (:`Completed`
          (message `/Game/Blueprints/Interfaces/BPI_HUD.DisplayNarrativeMessages` (`PlayerController.GetHUD` (`GameplayStatics.GetPlayerController` 0)))
          (`self.OnDisplayMessage`))))))

(fn `UserConstructionScript`
  (`parent.UserConstructionScript`))