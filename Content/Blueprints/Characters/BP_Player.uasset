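; Player Blueprint that picks up items through an interaction component and stores them in an inventory component.
; The CastInteractionTrace event has the interaction component run its trace.
; On a detected interaction, it gets the hit actor's pickable via CollectPickableMessage, adds it to the inventory, then looks it up by class without using the result.
; It also exposes its camera through a getter.
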(event `/Game/Blueprints/Interfaces/BPI_Player.CastInteractionTrace`
  (`/Game/Blueprints/Components/BP_InteractionComponent.CastTraceToInteract` (`self.BP_InteractionComponent`)))

(event `self.BP_InteractionComponent.OnDetectInteraction`
  (params (HitInfo :type "HitResult Structure"))
  (bind _pickable (message `/Game/Blueprints/Interfaces/BPI_Pickable.CollectPickable` (`.HitActor` (`GameplayStatics.BreakHitResult` HitInfo))))
  (`/Game/Blueprints/Components/BP_InventoryComponent.AddToInventory` (`self.BP_InventoryComponent`) _pickable)
  (`/Game/Blueprints/Components/BP_InventoryComponent.FindItemFromInventory` (`self.BP_InventoryComponent`) (`GameplayStatics.GetObjectClass` _pickable)))

(fn `GetCameraComponent`
  (returns (CameraComponent :type "CameraComponent Object Reference"))
  (return (`self.Camera`)))

(fn `UserConstructionScript`)